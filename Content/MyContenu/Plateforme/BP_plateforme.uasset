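; BP_plateforme is a one-time moving platform that carries the player while their input is locked.
; On box overlap, a `Trus` flag clears before the cast to BP_ThirdPersonCharacter, so any first overlapping actor uses up the trigger.
; The character is teleported to the `Tp` point, loses input, and InterpToMovement activates.
; After a delay equal to the movement's duration, input returns and a debug "Hello" prints.
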(event `self.Box.OnComponentBeginOverlap`
  (params (OverlappedComponent :type "PrimitiveComponent Object Reference") (OtherActor :type "Actor Object Reference") (OtherComp :type "PrimitiveComponent Object Reference") (OtherBodyIndex :type Integer) (bFromSweep :type Boolean) (SweepResult :type "HitResult Structure (by ref)"))
  ;[1 1 1] activation de la plaforme et le joueur ne peut bouger
  (if (`self.trus`)
    (set `self.trus` false)
    (bind _asbp_third_person_character (cast `/Game/ThirdPerson/Blueprints/BP_ThirdPersonCharacter` OtherActor))
    (`self.K2_TeleportTo` :`self` _asbp_third_person_character :`DestLocation` (`SceneComponent.K2_GetComponentLocation` (`self.tp`)))
    (`self.DisableInput` _asbp_third_person_character null)
    (`ActorComponent.Activate` (`self.InterpToMovement`) false)
    (`KismetSystemLibrary.Delay` (`InterpToMovementComponent.Duration` (`self.InterpToMovement`)))
    (`self.EnableInput` _asbp_third_person_character null)
    (`KismetSystemLibrary.PrintText` "Hello" true true (struct :`R` 1.0 :`B` 0.610647 :`A` 1.0))))

(fn `UserConstructionScript`)