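; BP_mine is a timed mine that explodes on its own a few seconds after spawning.
; On BeginPlay it waits, briefly flashes a hit overlay material on its Sphere, then applies radial damage centred on that sphere.
; It draws a debug sphere matching the damage radius and destroys itself.
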(event `self.ReceiveBeginPlay`
  ;[1 1 1] quand la Mine a Spawne
  (`KismetSystemLibrary.Delay` 4.0)
  ;;[1 0.02604 0.02604] Flasher Damage
  (`MeshComponent.SetOverlayMaterial` (`self.Sphere`) "/Game/MyContenu/Matériau/HIT.HIT")
  (`KismetSystemLibrary.Delay` 0.2)
  (`MeshComponent.SetOverlayMaterial` (`self.Sphere`) null)
  (`GameplayStatics.ApplyRadialDamage` :`BaseDamage` 50.0 :`Origin` (`SceneComponent.K2_GetComponentLocation` (`self.Sphere`)) :`DamageRadius` 500.0 :`DamageCauser` self :`InstigatedByController` null)
  (`KismetSystemLibrary.DrawDebugSphere` (`SceneComponent.K2_GetComponentLocation` (`self.Sphere`)) 500.0 12 (struct :`R` 1.0 :`G` 0.001778 :`B` 0.212378 :`A` 1.0))
  (`self.K2_DestroyActor`))

(fn `UserConstructionScript`)