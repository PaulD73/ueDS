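; Turret actor that turns toward and shoots the third-person player inside its sphere, and can be destroyed.
; A self-retriggering delay loop interpolates rotation until overlap ends, while a Delay throttles debug-drawn line traces.
; Any blocking hit damages the player, whatever was struck.
; Incoming damage flashes an overlay material, lowers HP and updates a camera-facing widget bar, shown only during SeeHPbar overlap.
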(event `retoure`
  (bind _arrow (`self.Arrow`))
  (bind _returnvalue (`SceneComponent.K2_GetComponentLocation` _arrow))
  ;[1 1 1] Si le joueur rentre dans la sphère de collision de la tourelle
  (bind _asbp_third_person_character (cast `/Game/ThirdPerson/Blueprints/BP_ThirdPersonCharacter` (stale `self.Sphere.OnComponentBeginOverlap` OtherActor) :!label _label))
  (if (`self.look`)
    (`KismetSystemLibrary.PrintText` "nop")
    (else
      ;;[1 0.698 0.1727] suis le joueur en rotation
      (`self.K2_SetActorRotation` (`KismetMathLibrary.RInterpTo` (`self.K2_GetActorRotation`) (`KismetMathLibrary.FindLookAtRotation` (`self.K2_GetActorLocation`) (`self.K2_GetActorLocation` _asbp_third_person_character)) (`GameplayStatics.GetWorldDeltaSeconds`) 13.0))
      ;;[1 0.09896 0.09896] Tire et applique des dégâts au joueur
      (`|ExecutionSequence`
        (:`then_0`
          (`KismetSystemLibrary.Delay` 0.3)
          (bind _outhit (`KismetSystemLibrary.LineTraceSingle` :`Start` _returnvalue :`End` (+ _returnvalue (* (`KismetMathLibrary.GetForwardVector` (`SceneComponent.K2_GetComponentRotation` _arrow)) (`KismetMathLibrary.Conv_DoubleToVector` 565.0))) :`TraceChannel` "TraceTypeQuery2" :`DrawDebugType` "ForDuration" :`DrawTime` 2.0))
          (if (`GameplayStatics.BreakHitResult` _outhit)
            (`GameplayStatics.ApplyDamage` _asbp_third_person_character 3.0)))
        (:`then_1`
          (`KismetSystemLibrary.Delay` 0.01)
          (`self.retoure`))))))

(event `self.Sphere.OnComponentBeginOverlap`
  (params (OverlappedComponent :type "PrimitiveComponent Object Reference") (OtherActor :type "Actor Object Reference") (OtherComp :type "PrimitiveComponent Object Reference") (OtherBodyIndex :type Integer) (bFromSweep :type Boolean) (SweepResult :type "HitResult Structure (by ref)"))
  ;[1 1 1] Si le joueur rentre dans la sphère de collision de la tourelle
  (set `self.look` false)
  (goto _label))

(event `self.Sphere.OnComponentEndOverlap`
  (params (OverlappedComponent :type "PrimitiveComponent Object Reference") (OtherActor :type "Actor Object Reference") (OtherComp :type "PrimitiveComponent Object Reference") (OtherBodyIndex :type Integer))
  ;[1 1 1] Si le joueur rentre dans la sphère de collision de la tourelle
  (cast `/Game/ThirdPerson/Blueprints/BP_ThirdPersonCharacter` OtherActor)
  (set `self.look` true))

(event `self.ReceiveAnyDamage`
  (params (Damage :type "Float (single-precision)") (DamageType :type "DamageType Object Reference") (InstigatedBy :type "Controller Object Reference") (DamageCauser :type "Actor Object Reference"))
  ;[1 1 1] subi des dégâts
  (`|ExecutionSequence`
    (:`then_0`
      ;;[1 0.02604 0.02604] Flasher Damage
      (`MeshComponent.SetOverlayMaterial` (`self.base`) "/Game/MyContenu/Matériau/HIT.HIT")
      (`KismetSystemLibrary.Delay` 0.2)
      (`MeshComponent.SetOverlayMaterial` (`self.base`) null))
    (:`then_1`
      ;;[0.3346 1 0.2989] Perdu des HP
      (set `self.HP` (- (`self.HP`) Damage))
      (bind _aswb_tourel_hp_bar (cast `/Game/MyContenu/Wedget/WB_tourelHpBar` (`WidgetComponent.GetWidget` (`self.Widget`))))
      (`/Game/MyContenu/Wedget/WB_tourelHpBar.UpBar` _aswb_tourel_hp_bar (`self.HP`))
      (if (<= (`self.HP`) 0.0)
        (`self.K2_DestroyActor`)))))

(event `self.ReceiveTick`
  (params (DeltaSeconds :type "Float (single-precision)"))
  ;[1 1 1] suis le joueur en rotation pour la bar HP de la tourel
  (`SceneComponent.K2_SetWorldRotation` (`self.Widget`) (`KismetMathLibrary.FindLookAtRotation` (`SceneComponent.K2_GetComponentLocation` (`self.Widget`)) (`SceneComponent.K2_GetComponentLocation` (`Actor.RootComponent` (`GameplayStatics.GetPlayerCameraManager` 0)))) false false))

(event `self.SeeHPbar.OnComponentBeginOverlap`
  (params (OverlappedComponent :type "PrimitiveComponent Object Reference") (OtherActor :type "Actor Object Reference") (OtherComp :type "PrimitiveComponent Object Reference") (OtherBodyIndex :type Integer) (bFromSweep :type Boolean) (SweepResult :type "HitResult Structure (by ref)"))
  ;[1 1 1] Quand et visible la bar d'HP
  (`SceneComponent.SetVisibility` (`self.Widget`) true false))

(event `self.SeeHPbar.OnComponentEndOverlap`
  (params (OverlappedComponent :type "PrimitiveComponent Object Reference") (OtherActor :type "Actor Object Reference") (OtherComp :type "PrimitiveComponent Object Reference") (OtherBodyIndex :type Integer))
  ;[1 1 1] Quand et visible la bar d'HP
  (`SceneComponent.SetVisibility` (`self.Widget`) false false))

(event `self.ReceiveBeginPlay`
  ;[1 1 1] Quand et visible la bar d'HP
  (`SceneComponent.SetVisibility` (`self.Widget`) false false)
  (bind _aswb_tourel_hp_bar (cast `/Game/MyContenu/Wedget/WB_tourelHpBar` (`WidgetComponent.GetUserWidgetObject` (`self.Widget`))))
  (set `/Game/MyContenu/Wedget/WB_tourelHpBar.Healh` (`self.HP`) _aswb_tourel_hp_bar))

(fn `UserConstructionScript`)